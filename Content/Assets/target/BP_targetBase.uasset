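; BP_targetBase is a shootable target actor that can only be destroyed once it has been revealed.
; BeginPlay sets its roll to StartXRotation, and the RevealTarget event sets the HasBeenReveled flag.
; When a FirstPersonProjectile hits the Target component while that flag is set, DoHit spawns an explosion, plays a break sound and destroys the actor.
; A delayed call to RevealTarget is left unconnected and never runs.
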(event `Reveal Target`
  (set `self.Has Been Reveled?` true))

(event `Do Hit`
  (bind _returnvalue (`self.K2_GetActorLocation`))
  (`GameplayStatics.SpawnEmitterAtLocation` "/Game/StarterContent/Particles/P_Explosion.P_Explosion" _returnvalue)
  (`GameplayStatics.PlaySoundAtLocation` "/Game/Gun_Sounds_Pro_HD_Remake/Wavs/Armor_Break_3.Armor_Break_3" _returnvalue (struct) 1.0 1.0 0.0 null null null)
  (`self.K2_DestroyActor`))

(event `self.Target.OnComponentHit`
  (params (HitComponent :type "PrimitiveComponent Object Reference") (OtherActor :type "Actor Object Reference") (OtherComp :type "PrimitiveComponent Object Reference") (NormalImpulse :type "Vector Structure") (Hit :type "HitResult Structure (by ref)"))
  (cast `/Game/VRExpansion/FirstPersonBP/FirstPersonBP/Blueprints/FirstPersonProjectile` OtherActor)
  (if (`self.Has Been Reveled?`)
    (`self.Do Hit`)))

(event `self.ReceiveBeginPlay`
  (bind (_returnvalue_roll _returnvalue_pitch _returnvalue_yaw) (`KismetMathLibrary.BreakRotator` (`self.K2_GetActorRotation`)))
  (`self.K2_SetActorRotation` (`KismetMathLibrary.MakeRotator` (`self.Start X Rotation`) _returnvalue_pitch _returnvalue_yaw)))

(fn `UserConstructionScript`)