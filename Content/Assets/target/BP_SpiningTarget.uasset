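; BP_SpiningTarget is a target variant that spins rapidly when hit before running its inherited hit response.
; DoHit sets HasBeenHit, waits one second, then calls the parent DoHit, so the parent behavior is delayed.
; While the flag is set, Tick adds frame-rate-independent local yaw to the Target component; this file never clears the flag.
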(event `self.Do Hit`
  (set `self.Has Been Hit?` true)
  (`KismetSystemLibrary.Delay` 1.0)
  (`parent.Do Hit`))

(event `self.ReceiveTick`
  (params (DeltaSeconds :type "Float (single-precision)"))
  (if (`self.Has Been Hit?`)
    (`SceneComponent.K2_AddLocalRotation` (`self.Target`) (`KismetMathLibrary.MakeRotator` 0.0 0.0 (* DeltaSeconds 2000.0)) false false)))

(fn `UserConstructionScript`
  (`parent.UserConstructionScript`))